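; EstrellaBP is a star actor that acts as the level goal, advancing the game when its Box is overlapped.
; The overlap, unfiltered by actor, reads LevelNow from the VariablesGI game instance to open NivelDos or NivelTres by name.
; On the third level it instead clears all widgets, shows the WG_VICTORIA victory screen and enables the mouse cursor.
; It never updates LevelNow itself, as its increment nodes are disconnected.
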(event `self.Box.OnComponentBeginOverlap`
  (params (OverlappedComponent :type "PrimitiveComponent Object Reference") (OtherActor :type "Actor Object Reference") (OtherComp :type "PrimitiveComponent Object Reference") (OtherBodyIndex :type Integer) (bFromSweep :type Boolean) (SweepResult :type "HitResult Structure (by ref)"))
  (bind _returnvalue (`GameplayStatics.GetPlayerController` 0))
  (bind _asvariables_gi (cast `/Game/Comunes/hud/VariablesGI` (`GameplayStatics.GetGameInstance`)))
  (switch `int` (`/Game/Comunes/hud/VariablesGI.LevelNow` _asvariables_gi)
    (:`1`
      (`GameplayStatics.OpenLevel` "NivelDos"))
    (:`2`
      (`GameplayStatics.OpenLevel` "NivelTres"))
    (:`3`
      (`WidgetLayoutLibrary.RemoveAllWidgets`)
      (bind _returnvalue_2 (`|CreateWidget` "/Game/NivelesJuego/menu_material/WG_VICTORIA.WG_VICTORIA_C" _returnvalue))
      (`UserWidget.AddToViewport` _returnvalue_2 0)
      (set `PlayerController.bShowMouseCursor` true _returnvalue))))

(fn `UserConstructionScript`)