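; Player actor for the main menu that moves itself between preset viewpoints for main, options, three character and play screens.
; Each Tick, Opciones selects the target location and rotation; while Navop is set, the Rot timeline lerps toward it from the current transform.
; On finish it snaps, clears Navop and spawns that screen's widget with the mouse cursor shown.
; BeginPlay checks the saveWorld1 slot, setting HaveWorld on the game instance and loading any save.
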(event `InitialSaveGame`
  (bind _returnvalue (`GameplayStatics.GetGameInstance`))
  (bind _returnvalue_2 (`GameplayStatics.DoesSaveGameExist` "saveWorld1"))
  (if _returnvalue_2
    (bind _asvariables_gi (cast `` _returnvalue))
    (set `/Game/NivelesJuego/menu_material/BP_PlayerMenu.haveWorld` true _asvariables_gi)
    (bind _returnvalue_3 (`GameplayStatics.LoadGameFromSlot` "saveWorld1"))
    (bind _asbp_save_game (cast `/Game/Comunes/Guardado/BP_SaveGame` _returnvalue_3))
    (set `self.BP_SaveGame` _asbp_save_game)
    (else
      (bind _asvariables_gi_2 (cast `` _returnvalue))
      (set `/Game/NivelesJuego/menu_material/BP_PlayerMenu.haveWorld` false _asvariables_gi_2))))

(event `self.ReceiveBeginPlay`
  (`self.InitialSaveGame`))

(event `self.ReceiveTick`
  (params (DeltaSeconds :type "Float (single-precision)"))
  (bind (_returnvalue_x _returnvalue_y _returnvalue_z) (`KismetMathLibrary.BreakVector` (`self.K2_GetActorLocation`)))
  (bind (_returnvalue_roll _returnvalue_pitch _returnvalue_yaw) (`KismetMathLibrary.BreakRotator` (`self.K2_GetActorRotation`)))
  (`self.VerificarOpcion`)
  (if (`self.navop`)
    (bind (_direction _rotar) (`Timeline|Rot` :!label _label)
      (:`Update`
        (`self.K2_SetActorLocationAndRotation` (`KismetMathLibrary.MakeVector` (`KismetMathLibrary.Lerp` _returnvalue_x (`self.PosX`) _rotar) (`KismetMathLibrary.Lerp` _returnvalue_y (`self.PosY`) _rotar) (`KismetMathLibrary.Lerp` _returnvalue_z (`self.PosZ`) _rotar)) (`KismetMathLibrary.MakeRotator` (`KismetMathLibrary.Lerp` _returnvalue_roll (`self.RotX`) _rotar) (`KismetMathLibrary.Lerp` _returnvalue_pitch (`self.RotY`) _rotar) (`KismetMathLibrary.Lerp` _returnvalue_yaw (`self.RotZ`) _rotar))))
      (:`Finished`
        (if (`self.navop`)
          (`self.K2_SetActorLocationAndRotation` (`KismetMathLibrary.MakeVector` (`self.PosX`) (`self.PosY`) (`self.PosZ`)) (`KismetMathLibrary.MakeRotator` (`self.RotX`) (`self.RotY`) (`self.RotZ`)))
          (set `self.navop` false)
          (`self.ResetHud`))))
    (else
      (goto _label :!via `PlayFromStart`))))

(fn `ResetHud`
  (bind _returnvalue (`GameplayStatics.GetPlayerController` 0))
  (switch `int` (`self.Opciones`)
    (:`Default`
      (`self.SetMenuP` :!label _label)
      (bind _returnvalue_2 (`|CreateWidget` "/Game/NivelesJuego/menu_material/WG_Menuprincipal.WG_Menuprincipal_C" _returnvalue))
      (`UserWidget.AddToViewport` _returnvalue_2 0))
    (:`0`
      (goto _label))
    (:`1`
      (`self.SetMenuP_Options`)
      (bind _returnvalue_3 (`|CreateWidget` "/Game/NivelesJuego/menu_material/WG_Menu_Opciones.WG_Menu_Opciones_C" _returnvalue))
      (`UserWidget.AddToViewport` _returnvalue_3 0))
    (:`2`
      (`self.SetMenuP_CH1`)
      (bind _returnvalue_4 (`|CreateWidget` "/Game/NivelesJuego/menu_material/WG_MenuPersonajes.WG_MenuPersonajes_C" _returnvalue :!label _label_2))
      (`UserWidget.AddToViewport` _returnvalue_4 0))
    (:`3`
      (`self.SetMenuP_CH2`)
      (goto _label_2))
    (:`4`
      (`self.SetMenuP_CH3`)
      (goto _label_2))
    (:`5`
      (`self.SetMenuP_Play`)
      (bind _returnvalue_5 (`|CreateWidget` "/Game/NivelesJuego/menu_material/WG_MenuPlay.WG_MenuPlay_C" _returnvalue))
      (`UserWidget.AddToViewport` _returnvalue_5 0)))
  (set `PlayerController.bShowMouseCursor` true _returnvalue))

(fn `SetMenuP`
  (set `self.RotX` 0.0)
  (set `self.RotY` 17.229396)
  (set `self.RotZ` 148.433296)
  (set `self.PosX` 3944.32476)
  (set `self.PosY` 4900.250256)
  (set `self.PosZ` 364.059994))

(fn `SetMenuP_CH1`
  (set `self.RotX` 0.0)
  (set `self.RotY` 17.229396)
  (set `self.RotZ` 48.433297)
  (set `self.PosX` 2494.32476)
  (set `self.PosY` 5160.250256)
  (set `self.PosZ` 884.059994))

(fn `SetMenuP_CH2`
  (set `self.RotX` 18.585285)
  (set `self.RotY` 12.064915)
  (set `self.RotZ` 31.552094)
  (set `self.PosX` 1744.32476)
  (set `self.PosY` 4410.250256)
  (set `self.PosZ` 424.059994))

(fn `SetMenuP_CH3`
  (set `self.RotX` 2.515749)
  (set `self.RotY` 36.064889)
  (set `self.RotZ` -41.963243)
  (set `self.PosX` 2084.32476)
  (set `self.PosY` 6440.250256)
  (set `self.PosZ` 404.059994))

(fn `SetMenuP_Options`
  (set `self.RotX` 15.025775)
  (set `self.RotY` -22.503992)
  (set `self.RotZ` -90.0)
  (set `self.PosX` 3444.32476)
  (set `self.PosY` 6850.250256)
  (set `self.PosZ` 1094.059994))

(fn `SetMenuP_Play`
  (set `self.RotX` 32.96495)
  (set `self.RotY` -20.917951)
  (set `self.RotZ` 47.278765)
  (set `self.PosX` 1744.32476)
  (set `self.PosY` 4410.250256)
  (set `self.PosZ` 884.059994))

(fn `UserConstructionScript`)

(fn `VerificarOpcion`
  (switch `int` (`self.Opciones`)
    (:`Default`
      (`self.SetMenuP` :!label _label))
    (:`0`
      (goto _label))
    (:`1`
      (`self.SetMenuP_Options`))
    (:`2`
      (`self.SetMenuP_CH1`))
    (:`3`
      (`self.SetMenuP_CH2`))
    (:`4`
      (`self.SetMenuP_CH3`))
    (:`5`
      (`self.SetMenuP_Play`))))